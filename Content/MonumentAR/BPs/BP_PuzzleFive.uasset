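; BP_PuzzleFive is a touch puzzle where three cubes must each be turned to a randomly chosen yaw, set on BeginPlay.
; Touching a cube turns it a quarter turn in timed steps, with InRotation blocking further touches meanwhile.
; CubeFunc compares its yaw to the stored target, swapping material and adjusting SolveNumber.
; When the counter reaches zero, Tick waits briefly, spawns BP_PuzzleSix in its place and destroys this actor.
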(event Custom|OnTouch
  (params (Hit :type Hit%20Result%20Structure))
  (bind _hitcomponent (Collision|BreakHitResult Hit))
  (bind _cube1 (Variables|Default|GetCube1))
  (bind _cube2 (Variables|Default|GetCube2))
  (bind _cube (Variables|Default|GetCube))
  (if (not (Variables|Default|GetinRotation))
    (if (== _cube _hitcomponent)
      (Utilities|RotateCube _cube)
      (CallFunction|CubeFunc _cube)
      (Variables|Default|SetinRotation false :!label _label)
      (elif (== _cube1 _hitcomponent)
        (Utilities|RotateCube _cube1)
        (CallFunction|CubeFunc _cube1)
        (goto _label)
        (elif (== _cube2 _hitcomponent)
          (Utilities|RotateCube _cube2)
          (CallFunction|CubeFunc _cube2)
          (goto _label))))))

(event EventBeginPlay
  (CallFunction|AddRandomUniqueButtoninSeq))

(event EventTick
  (params (DeltaSeconds :type Float%20%28single-precision%29))
  (if (Variables|Default|GetDestroy)
    (Utilities|FlowControl|DoOnce false
      (:Completed
        (Utilities|FlowControl|Delay 1.5)
        (Game|SpawnActorfromClass "/Game/MonumentAR/BPs/BP_PuzzleSix.BP_PuzzleSix_C" (Transformation|GetActorTransform) "Undefined" "MultiplyWithRoot" 0 0)
        (Actor|DestroyActor)))))

(event Input|ActionEvents|InputActionOneFingerAction
  (params (Key :type Key%20Structure :default "None")))

(fn ConstructionScript)

(fn ButtonFunc
  (params (button :type Static%20Mesh%20Component%20Object%20Reference)))

(fn AddRandomUniqueButtoninSeq
  (Utilities|Map|Add (Variables|Default|GetSeq) (Variables|Default|GetCube) (+ (Math|Random|RandomInteger 4) -1))
  (Utilities|Map|Add (Variables|Default|GetSeq) (Variables|Default|GetCube1) (+ (Math|Random|RandomInteger 4) -1))
  (Utilities|Map|Add (Variables|Default|GetSeq) (Variables|Default|GetCube2) (+ (Math|Random|RandomInteger 4) -1)))

(fn CubeFunc
  (params (Cube :type Static%20Mesh%20Component%20Object%20Reference))
  (if (== (Class|KismetMathLibrary|ToInt64(Integer) (.Value (Utilities|Map|Find (Variables|Default|GetSeq) Cube))) (Class|KismetMathLibrary|ToInt64(Float) (/ (.yaw (Variables|/Script/Engine.SceneComponent|GetRelativeRotation Cube)) 9e+01)))
    (bind _result (Math|Integer|DecrementInt (Variables|Default|GetSolveNumber))
      (:%20%20
        (Rendering|Material|SetMaterial Cube 0 "/Game/MonumentAR/Materials/ButtonMaterial_Inst3.ButtonMaterial_Inst3")
        (if (== _result 0)
          (Variables|Default|SetDestroy true))))
    (elif (== (Rendering|Material|GetMaterial Cube 0) "/Game/MonumentAR/Materials/ButtonMaterial_Inst3.ButtonMaterial_Inst3")
      (Rendering|Material|SetMaterial Cube 0 "/Game/MonumentAR/Materials/ButtonMaterial_Inst2.ButtonMaterial_Inst2")
      (Math|Integer|IncrementInt (Variables|Default|GetSolveNumber)))))