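; BP_PuzzleTwo is a puzzle stage in MonumentAR with four touchable button components that toggle between two materials.
; OnTouch matches the hit component to a button and passes it to ButtonFunc, which uses the current material as toggle state.
; Toggling on decrements SolveNumber and toggling off increments it.
; When the count reaches zero, the actor spawns BP_PuzzleThree at its own transform and destroys itself.
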(event Custom|OnTouch
  (params (Hit :type Hit%20Result%20Structure))
  (bind _hitcomponent (Collision|BreakHitResult Hit))
  (bind _button3 (Variables|Default|GetButton3))
  (bind _button (Variables|Default|GetButton))
  (bind _button1 (Variables|Default|GetButton1))
  (bind _button2 (Variables|Default|GetButton2))
  (if (== _button _hitcomponent)
    (CallFunction|ButtonFunc _button)
    (elif (== _button1 _hitcomponent)
      (CallFunction|ButtonFunc _button1)
      (elif (== _button2 _hitcomponent)
        (CallFunction|ButtonFunc _button2)
        (elif (== _hitcomponent _button3)
          (CallFunction|ButtonFunc _button3))))))

(fn ConstructionScript)

(fn ButtonFunc
  (params (Button :type Static%20Mesh%20Component%20Object%20Reference))
  (bind _solvenumber (Variables|Default|GetSolveNumber))
  (if (!= (Rendering|Material|GetMaterial Button 0) "/Game/MonumentAR/Materials/ButtonMaterial_Inst.ButtonMaterial_Inst")
    (Math|Integer|DecrementInt _solvenumber
      (:%20%20
        (if (== _solvenumber 0)
          (Game|SpawnActorfromClass "/Game/MonumentAR/BPs/BP_PuzzleThree.BP_PuzzleThree_C" (Transformation|GetActorTransform) "Undefined" "MultiplyWithRoot" 0 0)
          (Actor|DestroyActor)
          (else
            (Rendering|Material|SetMaterial Button 0 "/Game/MonumentAR/Materials/ButtonMaterial_Inst.ButtonMaterial_Inst")))))
    (else
      (Math|Integer|IncrementInt _solvenumber
        (:%20%20
          (Rendering|Material|SetMaterial Button 0 "/Game/MonumentAR/Materials/ButtonMaterial.ButtonMaterial"))))))