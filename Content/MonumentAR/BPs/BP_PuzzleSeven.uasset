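; BP_PuzzleSeven is a MonumentAR puzzle actor solved by repeatedly touching its cube.
; BeginPlay picks a random required touch count, and each OnTouch hit on the Cube component increments progress and shrinks the cube slightly.
; When progress matches the target, it spawns BP_WIn at its own transform and destroys itself.
; The construction script and ButtonFunc are empty.
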(event Custom|OnTouch
  (params (Hit :type Hit%20Result%20Structure))
  (bind _cube (Variables|Default|GetCube))
  (if (== (.HitComponent (Collision|BreakHitResult Hit)) (Variables|Default|GetCube))
    (Math|Integer|IncrementInt (Variables|Default|Getprogress)
      (:%20%20
        (Transformation|SetWorldScale3D _cube (* (Transformation|GetWorldScale _cube) "0.950000,0.950000,0.950000"))
        (if (== (Variables|Default|Getprogress) (Variables|Default|GetSolveNumber))
          (Game|SpawnActorfromClass "/Game/MonumentAR/BPs/BP_WIn.BP_WIn_C" (Transformation|GetActorTransform) "Undefined" "MultiplyWithRoot" 0 0)
          (Actor|DestroyActor))))))

(event EventBeginPlay
  (Variables|Default|SetSolveNumber (+ (Math|Random|RandomInteger 20) 10)))

(event Input|ActionEvents|InputActionOneFingerAction
  (params (Key :type Key%20Structure :default "None")))

(fn ConstructionScript)

(fn ButtonFunc)