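; BP_PuzzleSix is a two-stage touch puzzle in MonumentAR that spawns BP_PuzzleSeven in its place when solved.
; First, tapped cubes turn a quarter turn in timed steps and change material at their randomly chosen yaw.
; Once all three match, three buttons must be pressed in a random order generated at BeginPlay.
; A wrong press resets progress and changes the cube materials, which Tick restores after a delay, gating further button input.
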(event Custom|OnTouch
  (params (Hit :type Hit%20Result%20Structure))
  (bind _hitcomponent (Collision|BreakHitResult Hit))
  (bind _cube2 (Variables|Default|GetCube2))
  (bind _cube (Variables|Default|GetCube))
  (bind _button2 (Variables|Default|GetButton2))
  (bind _button1 (Variables|Default|GetButton1))
  (bind _button (Variables|Default|GetButton))
  (bind _cube1 (Variables|Default|GetCube1))
  (if (not (Variables|Default|GetButtonReady))
    (if (not (Variables|Default|GetinRotation))
      (if (== _cube _hitcomponent)
        (Utilities|RotateCube _cube)
        (CallFunction|CubeFunc _cube)
        (Variables|Default|SetinRotation false :!label _label)
        (elif (== _cube1 _hitcomponent)
          (Utilities|RotateCube _cube1)
          (CallFunction|CubeFunc _cube1)
          (goto _label)
          (elif (== _cube2 _hitcomponent)
            (Utilities|RotateCube _cube2)
            (CallFunction|CubeFunc _cube2)
            (goto _label)))))
    (elif (== (Rendering|Material|GetMaterial (Variables|Default|GetCube2) 0) "/Game/MonumentAR/Materials/ButtonMaterial_Inst3.ButtonMaterial_Inst3")
      (if (== _hitcomponent _button2)
        (CallFunction|ButtonFunc _button2)
        (elif (== _hitcomponent _button1)
          (CallFunction|ButtonFunc _button1)
          (elif (== _hitcomponent _button)
            (CallFunction|ButtonFunc _button)))))))

(event EventBeginPlay
  (CallFunction|Aaa)
  (CallFunction|AddRandomUniqueButtoninSeq :!label _label)
  (if (not (== (Utilities|Array|Length (Variables|Default|GetSeq_0)) (Variables|Default|GetSolveNumber)))
    (goto _label)))

(event EventTick
  (params (DeltaSeconds :type Float%20%28single-precision%29))
  (if (== (Rendering|Material|GetMaterial (Variables|Default|GetCube2) 0) "/Game/MonumentAR/Materials/ButtonMaterial_Inst1.ButtonMaterial_Inst1")
    (Utilities|FlowControl|Delay 1.0)
    (Rendering|Material|SetMaterial (Variables|Default|GetCube) 0 "/Game/MonumentAR/Materials/ButtonMaterial_Inst3.ButtonMaterial_Inst3")
    (Rendering|Material|SetMaterial (Variables|Default|GetCube1) 0 "/Game/MonumentAR/Materials/ButtonMaterial_Inst3.ButtonMaterial_Inst3")
    (Rendering|Material|SetMaterial (Variables|Default|GetCube2) 0 "/Game/MonumentAR/Materials/ButtonMaterial_Inst3.ButtonMaterial_Inst3")))

(fn ConstructionScript)

(fn Aaa
  (Utilities|Map|Add (Variables|Default|GetSeq) (Variables|Default|GetCube) (+ (Math|Random|RandomInteger 4) -1))
  (Utilities|Map|Add (Variables|Default|GetSeq) (Variables|Default|GetCube1) (+ (Math|Random|RandomInteger 4) -1))
  (Utilities|Map|Add (Variables|Default|GetSeq) (Variables|Default|GetCube2) (+ (Math|Random|RandomInteger 4) -1)))

(fn CubeFunc
  (params (Cube :type Static%20Mesh%20Component%20Object%20Reference))
  (if (== (Class|KismetMathLibrary|ToInt64(Integer) (.Value (Utilities|Map|Find (Variables|Default|GetSeq) Cube))) (Class|KismetMathLibrary|ToInt64(Float) (/ (.yaw (Variables|/Script/Engine.SceneComponent|GetRelativeRotation Cube)) 9e+01)))
    (bind _result (Math|Integer|DecrementInt (Variables|Default|GetSolveNumber))
      (:%20%20
        (Rendering|Material|SetMaterial Cube 0 "/Game/MonumentAR/Materials/ButtonMaterial_Inst3.ButtonMaterial_Inst3")
        (if (== _result 0)
          (Variables|Default|SetButtonReady true)
          (Rendering|Material|SetMaterial (Variables|Default|GetButton2) 0 "/Game/MonumentAR/Materials/ButtonMaterial.ButtonMaterial")
          (Rendering|Material|SetMaterial (Variables|Default|GetButton1) 0 "/Game/MonumentAR/Materials/ButtonMaterial.ButtonMaterial")
          (Rendering|Material|SetMaterial (Variables|Default|GetButton) 0 "/Game/MonumentAR/Materials/ButtonMaterial.ButtonMaterial")
          (Variables|Default|SetSolveNumber 3)
          (Variables|Default|Setprogress 0))))
    (elif (== (Rendering|Material|GetMaterial Cube 0) "/Game/MonumentAR/Materials/ButtonMaterial_Inst3.ButtonMaterial_Inst3")
      (Rendering|Material|SetMaterial Cube 0 "/Game/MonumentAR/Materials/ButtonMaterial_Inst2.ButtonMaterial_Inst2")
      (Math|Integer|IncrementInt (Variables|Default|GetSolveNumber)))))

(fn AddRandomUniqueButtoninSeq
  (bind _seq_0 (Variables|Default|GetSeq_0))
  (switch int (Math|Random|RandomInteger 3)
    (:0
      (Utilities|Array|AddUnique _seq_0 (Variables|Default|GetButton)))
    (:1
      (Utilities|Array|AddUnique _seq_0 (Variables|Default|GetButton1)))
    (:2
      (Utilities|Array|AddUnique _seq_0 (Variables|Default|GetButton2)))))

(fn ButtonFunc
  (params (button :type Static%20Mesh%20Component%20Object%20Reference))
  (if (== button (Utilities|Array|Get(acopy) (Variables|Default|GetSeq_0) (Variables|Default|Getprogress)))
    (Math|Integer|IncrementInt (Variables|Default|Getprogress)
      (:%20%20
        (Rendering|Material|SetMaterial button 0 "/Game/MonumentAR/Materials/ButtonMaterial_Inst.ButtonMaterial_Inst")
        (if (== (Variables|Default|Getprogress) (Variables|Default|GetSolveNumber))
          (Game|SpawnActorfromClass "/Game/MonumentAR/BPs/BP_PuzzleSeven.BP_PuzzleSeven_C" (Transformation|GetActorTransform) "Undefined" "MultiplyWithRoot" 0 0)
          (Actor|DestroyActor))))
    (else
      (Rendering|Material|SetMaterial (Variables|Default|GetButton) 0 "/Game/MonumentAR/Materials/ButtonMaterial.ButtonMaterial")
      (Rendering|Material|SetMaterial (Variables|Default|GetButton1) 0 "/Game/MonumentAR/Materials/ButtonMaterial.ButtonMaterial")
      (Rendering|Material|SetMaterial (Variables|Default|GetButton2) 0 "/Game/MonumentAR/Materials/ButtonMaterial.ButtonMaterial")
      (Variables|Default|Setprogress 0)
      (Rendering|Material|SetMaterial (Variables|Default|GetCube) 0 "/Game/MonumentAR/Materials/ButtonMaterial_Inst1.ButtonMaterial_Inst1")
      (Rendering|Material|SetMaterial (Variables|Default|GetCube1) 0 "/Game/MonumentAR/Materials/ButtonMaterial_Inst1.ButtonMaterial_Inst1")
      (Rendering|Material|SetMaterial (Variables|Default|GetCube2) 0 "/Game/MonumentAR/Materials/ButtonMaterial_Inst1.ButtonMaterial_Inst1"))))