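; BP_PuzzleThree is a touch puzzle in MonumentAR where three buttons must be pressed in a random order.
; BeginPlay builds the sequence by adding random unique buttons until it reaches SolveNumber.
; Correct touches highlight buttons and advance progress; completion spawns BP_PuzzleFour in its place.
; Mistakes reset progress and switch the cube's material, which doubles as an input lock until Tick restores it after a delay.
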(event Custom|OnTouch
  (params (Hit :type Hit%20Result%20Structure))
  (bind _hitcomponent (Collision|BreakHitResult Hit))
  (bind _button (Variables|Default|GetButton))
  (bind _button1 (Variables|Default|GetButton1))
  (bind _button2 (Variables|Default|GetButton2))
  (if (== (Rendering|Material|GetMaterial (Variables|Default|GetCube) 0) "/Game/MonumentAR/Materials/ButtonMaterial_Inst2.ButtonMaterial_Inst2")
    (if (== _button _hitcomponent)
      (CallFunction|ButtonFunc _button)
      (elif (== _button1 _hitcomponent)
        (CallFunction|ButtonFunc _button1)
        (elif (== _button2 _hitcomponent)
          (CallFunction|ButtonFunc _button2))))))

(event EventBeginPlay
  (CallFunction|AddRandomUniqueButtoninSeq :!label _label)
  (if (not (== (Utilities|Array|Length (Variables|Default|GetSeq)) (Variables|Default|GetSolveNumber)))
    (goto _label)))

(event EventTick
  (params (DeltaSeconds :type Float%20%28single-precision%29))
  (if (== (Rendering|Material|GetMaterial (Variables|Default|GetCube) 0) "/Game/MonumentAR/Materials/ButtonMaterial_Inst1.ButtonMaterial_Inst1")
    (Utilities|FlowControl|Delay 1.0)
    (Rendering|Material|SetMaterial (Variables|Default|GetCube) 0 "/Game/MonumentAR/Materials/ButtonMaterial_Inst2.ButtonMaterial_Inst2")))

(event Input|ActionEvents|InputActionOneFingerAction
  (params (Key :type Key%20Structure :default "None")))

(fn ConstructionScript)

(fn ButtonFunc
  (params (button :type Static%20Mesh%20Component%20Object%20Reference))
  (if (== button (Utilities|Array|Get(acopy) (Variables|Default|GetSeq) (Variables|Default|Getprogress)))
    (Math|Integer|IncrementInt (Variables|Default|Getprogress)
      (:%20%20
        (Rendering|Material|SetMaterial button 0 "/Game/MonumentAR/Materials/ButtonMaterial_Inst.ButtonMaterial_Inst")
        (if (== (Variables|Default|Getprogress) (Variables|Default|GetSolveNumber))
          (Game|SpawnActorfromClass "/Game/MonumentAR/BPs/BP_PuzzleFour.BP_PuzzleFour_C" (Transformation|GetActorTransform) "Undefined" "MultiplyWithRoot" 0 0)
          (Actor|DestroyActor))))
    (else
      (Rendering|Material|SetMaterial (Variables|Default|GetButton) 0 "/Game/MonumentAR/Materials/ButtonMaterial.ButtonMaterial")
      (Rendering|Material|SetMaterial (Variables|Default|GetButton1) 0 "/Game/MonumentAR/Materials/ButtonMaterial.ButtonMaterial")
      (Rendering|Material|SetMaterial (Variables|Default|GetButton2) 0 "/Game/MonumentAR/Materials/ButtonMaterial.ButtonMaterial")
      (Variables|Default|Setprogress 0)
      (Rendering|Material|SetMaterial (Variables|Default|GetCube) 0 "/Game/MonumentAR/Materials/ButtonMaterial_Inst1.ButtonMaterial_Inst1"))))

(fn AddRandomUniqueButtoninSeq
  (switch int (Math|Random|RandomInteger 3)
    (:0
      (Utilities|Array|AddUnique (Variables|Default|GetSeq) (Variables|Default|GetButton)))
    (:1
      (Utilities|Array|AddUnique (Variables|Default|GetSeq) (Variables|Default|GetButton1)))
    (:2
      (Utilities|Array|AddUnique (Variables|Default|GetSeq) (Variables|Default|GetButton2)))))